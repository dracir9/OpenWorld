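; WorldManager_BP is a world manager Blueprint that generates a runtime mesh in its construction script.
; AddTriangles turns the Values array into vertices and triangles, which RuntimeMesh builds into a mesh section.
; A dynamic instance of the Grass material is created on that mesh and stored in Mat.
; Disconnected nodes for editing Values and setting a cobblestone texture never run.
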(fn `UserConstructionScript`
  (bind (_vertex _triangles) (`self.AddTriangles` (`self.Values`)))
  (`RuntimeMeshComponent.CreateMeshSection_Blueprint` :`self` (`self.RuntimeMesh`) :`Vertices` _vertex :`Triangles` _triangles)
  (bind _returnvalue (`PrimitiveComponent.CreateDynamicMaterialInstance` (`self.RuntimeMesh`) 0 "/Game/Materials/Grass.Grass"))
  (bind _output_get (set `self.Mat` _returnvalue)))