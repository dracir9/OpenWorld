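; Player controller for voxel editing, with Wait, Remove and Add modes selected by number keys or cycled with mouse wheel up.
; Outside Wait, Tick line-traces from the camera and moves a preview cube to a FloorVector location, offset along the hit normal when adding.
; Left click writes that voxel through the WorldGameMode_BP, cached as WorldManager.
; It also triggers debug properties on BeginPlay and F6, and caps FPS in its construction script.
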(event `Key|MouseScrollUp`
  (params (Key :type "Key Structure"))
  (bind _state (`self.State`))
  (:`Pressed`
    (bind _output_get (set `self.State` (cast `/Game/State` (select `bool` (`|EnumEquality` _state "NewEnumerator2") :`false` (+ _state 1)))))
    (`KismetSystemLibrary.PrintString` (`|GetEnumeratorNameAsString` _output_get))))

(event `self.ReceiveBeginPlay`
  (bind _asworld_game_mode_bp (cast `/Game/GameBP/WorldGameMode_BP` (`GameplayStatics.GetGameMode`)))
  (bind _output_get (set `self.WorldManager` _asworld_game_mode_bp))
  (`/Game/GameBP/WorldGameMode_BP.ShowDebugProperties` _output_get))

(event `Key|One`
  (params (Key :type "Key Structure"))
  (:`Pressed`
    (set `self.State` "NewEnumerator0")))

(event `Key|Two`
  (params (Key :type "Key Structure"))
  (:`Pressed`
    (set `self.State` "NewEnumerator1")))

(event `self.ReceiveTick`
  (params (DeltaSeconds :type "Float (single-precision)"))
  (bind _returnvalue (`GameplayStatics.GetPlayerCameraManager` 0))
  (bind _returnvalue_2 (`PlayerCameraManager.GetCameraLocation` _returnvalue))
  (bind _voxelsize (`WorldGameMode.VoxelSize` (`self.WorldManager`)))
  (bind _returnvalue_3 (`KismetMathLibrary.Conv_IntToDouble` _voxelsize))
  (if (not (`|EnumEquality` (`self.State`) "NewEnumerator0"))
    (bind (_outhit _returnvalue_4) (`KismetSystemLibrary.LineTraceSingle` _returnvalue_2 (+ _returnvalue_2 (* (`self.GetActorForwardVector` _returnvalue) 1000)) "TraceTypeQuery1" false (`|MakeArray` (`self.Cube`) :!type "Actor Object Reference") "None" true (struct :`R` 1.0 :`A` 1.0) (struct :`G` 1.0 :`A` 1.0) 100.0))
    (if _returnvalue_4
      (bind (_bblockinghit _binitialoverlap _time _distance _location _impactpoint _normal) (`GameplayStatics.BreakHitResult` _outhit))
      (bind _output_get (set `self.Location` (select `/Game/State` (`self.State`) :`NewEnumerator1` (`self.FloorVector` _location _returnvalue_3) :`NewEnumerator2` (`self.FloorVector` (+ _location (* _normal (/ (`KismetMathLibrary.Conv_IntToDouble` _voxelsize) 1.0))) _returnvalue_3))))
      (`/Engine/EditorBlueprintResources/StandardMacros.IsValid` (`self.Cube`)
        (:`Is Valid`
          (bind _returnvalue_5 (`KismetMathLibrary.MakeTransform` _output_get (struct) (0.5 0.5 0.5)))
          (`self.K2_SetActorTransform` (`self.Cube`) _returnvalue_5 false false))
        (:`Is Not Valid`
          (bind _returnvalue_6 (`|SpawnActorFromClass` "/Game/GameBP/Cube.Cube_C" _returnvalue_5 "Undefined" "OverrideRootScale" null null))
          (set `self.Cube` _returnvalue_6))))))

(event `Key|Three`
  (params (Key :type "Key Structure"))
  (:`Pressed`
    (set `self.State` "NewEnumerator2")))

(event `Key|F6`
  (params (Key :type "Key Structure"))
  (:`Pressed`
    (`/Game/GameBP/WorldGameMode_BP.ShowDebugProperties` (`self.WorldManager`))))

(event `Key|LeftMouseButton`
  (params (Key :type "Key Structure"))
  (:`Pressed`
    (switch `/Game/State` (`self.State`)
      (:`NewEnumerator1`
        (bind _returnvalue (`WorldGameMode.SetVoxelFromWorld` (`self.WorldManager`) (`self.Location`) 0))
        (`KismetSystemLibrary.PrintString` (`KismetStringLibrary.Conv_BoolToString` _returnvalue)))
      (:`NewEnumerator2`
        (bind _returnvalue_2 (`WorldGameMode.SetVoxelFromWorld` (`self.WorldManager`) (`self.Location`) 2))
        (`KismetSystemLibrary.PrintString` (`KismetStringLibrary.Conv_BoolToString` _returnvalue_2))))))

(fn `UserConstructionScript`
  (`KismetSystemLibrary.ExecuteConsoleCommand` "t.maxfps 30"))