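; World game mode that provides a debug overlay toggle, a frame rate cap and a world noise source.
; ShowDebugProperties lazily creates the Debug_WB widget, adds it to the viewport, then toggles its visibility on later calls.
; The construction script caps the frame rate through a console command.
; CalculateNoise returns a newly created, fixed-seed simplex FBM noise generator; its consumers are outside this Blueprint.
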(event `ShowDebugProperties`
  (bind _debug_wb (`self.Debug WB`))
  (`/Engine/EditorBlueprintResources/StandardMacros.IsValid` (`self.Debug WB`)
    (:`Is Valid`
      (if (`Widget.IsInViewport` _debug_wb)
        (if (`Widget.IsVisible` _debug_wb)
          (`Widget.SetVisibility` _debug_wb "Hidden")
          (else
            (`Widget.SetVisibility` _debug_wb "Visible")))
        (else
          (`UserWidget.AddToViewport` _debug_wb 0 :!label _label))))
    (:`Is Not Valid`
      (bind _returnvalue (`|CreateWidget` "/Game/GameBP/Debug_WB.Debug_WB_C" (`GameplayStatics.GetPlayerController` 0)))
      (set `self.Debug WB` _returnvalue)
      (goto _label))))

(fn `CalculateNoise`
  (returns (ReturnValue :type "UFNNoiseGenerator Object Reference"))
  (return (`UFNBlueprintFunctionLibrary.CreateNoiseGenerator` self "Simplex" "Euclidean" "CellValue" "FBM" "InterpLinear" 1234 4 0.0001)))

(fn `UserConstructionScript`
  (`KismetSystemLibrary.ExecuteConsoleCommand` "t.maxfps 30"))